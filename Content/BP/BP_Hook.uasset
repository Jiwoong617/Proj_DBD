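; BP_Hook is a hook actor that a target, presumably the player, can be hung from.
; GetHookingPoint exposes the world location of its HookingPos component.
; HookPlayer attaches the passed component to a skeletal mesh socket, snapping location and rotation while keeping world scale.
; HangEvent blends the first player controller's view to the hook actor; the default BeginPlay, overlap and Tick events are unused.
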(event Custom|HangEvent
  (Game|Player|SetViewTargetwithBlend (Game|GetPlayerController 0) self 1.0 "VTBlend_Linear" 0.0 false))

(event EventBeginPlay)

(event Collision|EventActorBeginOverlap
  (params (OtherActor :type Actor%20Object%20Reference)))

(event EventTick
  (params (DeltaSeconds :type Float%20%28single-precision%29)))

(fn ConstructionScript)

(fn GetHookingPoint
  (return (Transformation|GetWorldLocation (Variables|Default|GetHookingPos))))

(fn HookPlayer
  (params (HookTarget :type Actor%20Object%20Reference))
  (Transformation|AttachComponentToComponent HookTarget (Variables|Default|GetSkeletalMesh) (Variables|Default|GetHookSocketName) "SnapToTarget" "SnapToTarget" "KeepWorld" true))