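; Escape room actor that serves as the end room, where a survivor reaches safety.
; On BeginPlay it registers itself with GM_MainGame through SetEndRoom.
; DoorOpen plays a positional sound and swings the door open with a yaw timeline.
; When a BP_SurvivorCharacter enters the box, it sets IsSurvive on the game instance and, after a short delay, switches the game mode's state.
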(event OnComponentBeginOverlap(Box)
  (params (OverlappedComponent :type Primitive%20Component%20Object%20Reference) (OtherActor :type Actor%20Object%20Reference) (OtherComp :type Primitive%20Component%20Object%20Reference) (OtherBodyIndex :type Integer) (bFromSweep :type Boolean) (SweepResult :type Hit%20Result%20Structure%20%28by%20ref%29))
  (Utilities|Casting|CastToBP_SurvivorCharacter OtherActor)
  (bind _asgi_game_instance (Utilities|Casting|CastToGI_GameInstance (Game|GetGameInstance)))
  (Variables|/Game/BP/GI_GameInstance.GI_GameInstance_C|SetIsSurvive _asgi_game_instance true)
  (Utilities|FlowControl|Delay 1.0)
  (bind _asgm_main_game (Utilities|Casting|CastToGM_MainGame (Game|GetGameMode)))
  (Default|SwtichGameState _asgm_main_game "NewEnumerator2"))

(event Custom|DoorOpen
  (bind _door (Variables|Default|GetDoor))
  (Audio|SpawnSoundatLocation "/Game/Sound/Door.Door" (Transformation|GetWorldLocation _door) "0, 0, 0" 1.0 1.0 0.0 "/Game/Sound/MySoundAttention.MySoundAttention" 0)
  (bind _doorrotation (Timeline|OpenDoor Play)
    (:Update
      (Transformation|SetRelativeRotation _door (Math|Rotator|MakeRotator 0.0 0.0 _doorrotation) false false))))

(event EventBeginPlay
  (bind _asgm_main_game (Utilities|Casting|CastToGM_MainGame (Game|GetGameMode)))
  (Default|SetEndRoom _asgm_main_game self))

(event Collision|EventActorBeginOverlap
  (params (OtherActor :type Actor%20Object%20Reference)))

(event EventTick
  (params (DeltaSeconds :type Float%20%28single-precision%29)))

(fn ConstructionScript)