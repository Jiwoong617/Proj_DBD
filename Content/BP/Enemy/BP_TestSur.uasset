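; BP_TestSur is an enemy-folder child Blueprint that acts as a survivor whose lifetime is tracked in the game instance.
; While it is not Dead, each Tick calls AddSurviveTime on GI_GameInstance after running the parent logic.
; TakeDmg runs the parent's damage handling, then clears IsSurvive on the game instance if Dead.
; BloodStain0 traces downward and spawns a randomly sized blood decal aligned to the impact normal.
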(event EventBeginPlay
  (|CallParentFunction))

(event Collision|EventActorBeginOverlap
  (params (OtherActor :type Actor%20Object%20Reference)))

(event EventTick
  (params (DeltaSeconds :type Float%20%28single-precision%29))
  (|CallParentFunction DeltaSeconds)
  (if (not (Variables|Default|GetDead))
    (bind _asgi_game_instance (Utilities|Casting|CastToGI_GameInstance (Game|GetGameInstance)))
    (Default|AddSurviveTime _asgi_game_instance)))

(fn ConstructionScript
  (|CallParentFunction))

(fn BloodStain0
  (bind _returnvalue (Transformation|GetActorLocation))
  (bind _outhit (Collision|LineTraceByChannel _returnvalue (+ _returnvalue (* (Transformation|GetActorUpVector) -100)) "TraceTypeQuery1" false 0 "None"))
  (Rendering|Decal|SpawnDecalatLocation "/Game/Materials/M_BloodStain.M_BloodStain" (Math|Vector|MakeVector 1.0 (Math|Random|RandomFloatinRange 1e+01 3e+01) (Math|Random|RandomFloatinRange 1e+01 3e+01)) (.Location (Collision|BreakHitResult _outhit)) (Math|Rotator|MakeRotfromX (.ImpactNormal (Collision|BreakHitResult _outhit))) 0.0))

(fn TakeDmg
  (params (Damage :type Integer))
  (|CallParentFunction Damage)
  (if (Variables|Default|GetDead)
    (bind _asgi_game_instance (Utilities|Casting|CastToGI_GameInstance (Game|GetGameInstance)))
    (Variables|/Game/BP/GI_GameInstance.GI_GameInstance_C|SetIsSurvive _asgi_game_instance false)))