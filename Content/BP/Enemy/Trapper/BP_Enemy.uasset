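; Killer enemy that roams, chases and attacks the survivor, then carries the dead player to a hook.
; A Tick-driven state machine also handles flashlight stuns and kicking interactive obstacles.
; Detection combines a view-cone dot product, throttled box traces and a proximity overlap.
; Roaming and chasing set velocity directly, hook trips use AI MoveTo, and attacks use a socketed weapon with a cooldown slowdown.
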(event OnComponentBeginOverlap(DetectNearPlayer)
  (params (OverlappedComponent :type Primitive%20Component%20Object%20Reference) (OtherActor :type Actor%20Object%20Reference) (OtherComp :type Primitive%20Component%20Object%20Reference) (OtherBodyIndex :type Integer) (bFromSweep :type Boolean) (SweepResult :type Hit%20Result%20Structure%20%28by%20ref%29))
  (Utilities|Casting|CastToBP_SurvivorCharacter OtherActor)
  (Variables|Default|SetIsPayerNear true))

(event OnComponentEndOverlap(DetectNearPlayer)
  (params (OverlappedComponent :type Primitive%20Component%20Object%20Reference) (OtherActor :type Actor%20Object%20Reference) (OtherComp :type Primitive%20Component%20Object%20Reference) (OtherBodyIndex :type Integer))
  (Utilities|Casting|CastToBP_SurvivorCharacter OtherActor)
  (Variables|Default|SetIsPayerNear false))

(event EventBeginPlay
  (CallFunction|Init))

(event EventTick
  (params (DeltaSeconds :type Float%20%28single-precision%29))
  (if (Variables|Default|GetIsStun)
    _
    (else
      (CallFunction|AttackCoolDown)
      (bind _isplayeronsight (CallFunction|IsPlayeronSight))
      (CallFunction|CheckinFront (Variables|Default|GetSightDistance) _isplayeronsight)
      (Variables|Default|SetIsFindPlayer (or (Variables|Default|GetIsLookingPlayer) (Variables|Default|GetIsPayerNear)))
      (CallFunction|CheckPlayerDead)))
  (switch Utilities|FlowControl|Switch|SwitchonEState (Variables|Default|GetPState)
    (:NewEnumerator0
      (CallFunction|OnIdle)
      (Development|PrintString (Utilities|String|EnumtoString (Variables|Default|GetPState)) true true "(R=0.000000,G=0.660000,B=1.000000,A=1.000000)" 2.0 "char" :!label _label))
    (:NewEnumerator1
      (CallFunction|OnMove)
      (goto _label))
    (:NewEnumerator2
      (CallFunction|OnAttack)
      (goto _label))
    (:NewEnumerator4
      (CallFunction|OnStun)
      (goto _label))
    (:NewEnumerator5
      (CallFunction|OnKick)
      (goto _label))
    (:NewEnumerator6
      (CallFunction|OnPlayerDead)
      (goto _label))
    (:NewEnumerator7
      (CallFunction|OnHook))))

(fn ConstructionScript
  (|CallParentFunction))

(fn Init
  (Variables|Default|SetPState "NewEnumerator0")
  (bind _returnvalue (Actor|GetActorOfClass "/Game/BP/Survivor/BP_SurvivorCharacter.BP_SurvivorCharacter_C"))
  (Variables|Default|SetPlayer _returnvalue)
  (bind _returnvalue_2 (Game|SpawnActorfromClass "/Game/BP/Enemy/BP_EnemyWeapon.BP_EnemyWeapon_C" (Math|Transform|MakeTransform "0, 0, 0") "Undefined" "MultiplyWithRoot" 0 0))
  (bind _output_get (Variables|Default|SetWeapon _returnvalue_2))
  (Variables|/Game/BP/Enemy/BP_EnemyWeapon.BP_EnemyWeapon_C|SetWeaponOwner _output_get self)
  (Transformation|AttachComponentToComponent _output_get (Variables|Character|GetMesh) "R_Socket" "SnapToTarget" "SnapToTarget" "SnapToTarget" true)
  (bind _returnvalue_3 (Actor|GetActorOfClass "/Game/BP/BP_Hook.BP_Hook_C"))
  (Variables|Default|SetHook _returnvalue_3))

(fn MoveActor
  (params (Dir :type Vector))
  (bind _returnvalue (Utilities|Time|GetWorldDeltaSeconds))
  (bind _returnvalue_2 (Transformation|GetActorRotation))
  (bind _returnvalue_3 (Transformation|GetActorLocation))
  (bind _returnvalue_4 (Math|Rotator|FindLookatRotation _returnvalue_3 Dir))
  (if (< (Math|Vector|Distance(Vector) (Variables|Default|GetDestination) (Transformation|GetActorLocation)) (Variables|Default|GetReachBias))
    (Transformation|SetActorRotation (Math|Interpolation|RInterpTo _returnvalue_2 _returnvalue_4 _returnvalue 5.0))
    (else
      (Transformation|SetActorRotation (Math|Interpolation|RInterpTo _returnvalue_2 _returnvalue_4 _returnvalue 1e+01))
      (Variables|/Script/Engine.MovementComponent|SetVelocity (Variables|Character|GetCharacterMovement) (* (Math|Vector|Normalize (- Dir (Transformation|GetActorLocation))) (Variables|Default|GetSpeed))))))

(fn MoveActorUsingAI
  (params (Destination :type Vector))
  (AI|Navigation|MovetoLocation (AI|GetAIController self) Destination 1e+01 true true true true 0))

(fn SetRandomPosition
  (bind _returnvalue (Transformation|GetActorLocation))
  (bind _returnvalue_2 (Math|Random|RandomUnitVector))
  (bind _returnvalue_3 (Math|Random|RandomFloatinRange 1.5e+03 2e+03))
  (bind _returnvalue_4 (* (Math|Vector|MakeVector (.x _returnvalue_2) (.y _returnvalue_2) 0.0) _returnvalue_3))
  (bind _returnvalue_5 (+ _returnvalue _returnvalue_4))
  (if (Math|Vector|VectorIsZero (Variables|Default|GetDestination))
    (Variables|Default|SetDestination _returnvalue_5)
    (Development|PrintString (Utilities|String|ToString(Vector) _returnvalue_5) true true "(R=0.000000,G=0.660000,B=1.000000,A=1.000000)" 2.0 "NEw")))

(fn OnIdle
  (if (Variables|Default|GetIsFindPlayer)
    (Variables|Default|SetPState "NewEnumerator2")
    (else
      (CallFunction|SetRandomPosition)
      (Variables|Default|SetPState "NewEnumerator1"))))

(fn OnMove
  (if (Variables|Default|GetIsFindPlayer)
    (Variables|Default|SetPState "NewEnumerator2")
    (else
      (CallFunction|MoveActor (Variables|Default|GetDestination))
      (bind _isreached (CallFunction|CheckActorReach))
      (if _isreached
        (Variables|Default|SetDestination "0, 0, 0")
        (CallFunction|SetRandomPosition)))))

(fn OnAttack
  (bind _player (Variables|Default|GetPlayer))
  (bind _returnvalue (Transformation|GetActorLocation _player))
  (if (Variables|Default|GetIsFindPlayer)
    (bind _output_get (Variables|Default|SetDestination (Math|Vector|MakeVector (.x _returnvalue) (.y _returnvalue) (.z (Transformation|GetActorLocation)))))
    (CallFunction|MoveActor _output_get)
    (bind _isreached (CallFunction|CheckActorReach))
    (if (Math|Boolean|ANDBoolean _isreached (Variables|Default|GetCanAttack) (not (Variables|Default|GetIsAttacking)))
      (CallFunction|AttackFunc))
    (else
      (Variables|Default|SetPState "NewEnumerator0"))))

(fn OnStun
  (bind _output_get (Variables|Default|SetStunTimer (+ (Variables|Default|GetStunTimer) (Utilities|Time|GetWorldDeltaSeconds))))
  (if (> _output_get 1.0)
    (Variables|Default|SetPState "NewEnumerator0")
    (Variables|Default|SetIsStun false)
    (Variables|Default|SetStunTimer 0.0)))

(fn OnKick
  (if (not (Variables|Default|GetIsKicking))
    (Variables|Default|SetIsKicking true)
    (Animation|PlayAnimMontage "/Game/BP/ABP/Kicking_Montage.Kicking_Montage" 1.0 "None")))

(fn OnPlayerDead
  (if (Variables|Default|GetIsCarrying)
    (if (Variables|Default|GetIsCarryPlayer)
      (Variables|Default|SetPState "NewEnumerator7"))
    (else
      (Variables|Default|SetIsCarrying true)
      (Animation|PlayAnimMontage "/Game/BP/ABP/Lifting_Montage.Lifting_Montage" 1.0 "None")
      (bind _hookingpoint (Default|GetHookingPoint (Variables|Default|GetHook)))
      (Variables|Default|SetDestination _hookingpoint))))

(fn OnHook
  (CallFunction|MoveActorUsingAI (Variables|Default|GetDestination))
  (if (< (Math|Vector|Distance(Vector) (Transformation|GetActorLocation) (Variables|Default|GetDestination)) (Variables|Default|GetReachBias))
    (Default|HookPlayer (Variables|Default|GetHook) (Variables|Default|GetPlayer))
    (CallFunction|ResetBoolDatas)
    (Variables|Default|SetPState "NewEnumerator0")))

(fn IsPlayeronSight
  (bind _returnvalue (Transformation|GetActorLocation))
  (bind _player (Variables|Default|GetPlayer))
  (bind _returnvalue_2 (Transformation|GetActorLocation _player))
  (return (and (> (Math|Vector|DotProduct (Math|Vector|Normalize (- _returnvalue_2 _returnvalue)) (Transformation|GetActorForwardVector)) (Math|Trig|Cos(Degrees) (Variables|Default|GetSightRadius))) (< (Math|Vector|Distance(Vector) _returnvalue_2 _returnvalue) (Variables|Default|GetSightDistance)))))

(fn CheckActorReach
  (return (< (Math|Vector|Distance(Vector) (Variables|Default|GetDestination) (Transformation|GetActorLocation)) (Variables|Default|GetReachBias))))

(fn AttackCoolDown
  (if (and (not (Variables|Default|GetCanAttack)) (not (Variables|Default|GetIsAttacking)))
    (bind _output_get (Variables|Default|SetAttackDelayTimer (- (Variables|Default|GetAttackDelayTimer) (Utilities|Time|GetWorldDeltaSeconds))))
    (if (< _output_get 0.0)
      (Variables|Default|SetCanAttack true)
      (Variables|Default|SetSpeed (/ (Variables|Default|GetSpeed) (Variables|Default|GetSpeedDecreaseMultiplyer))))))

(fn AttackFunc
  (Variables|Default|SetAttackDelayTimer (Variables|Default|GetAttackFailDelay))
  (Variables|Default|SetSpeed (* (Variables|Default|GetSpeed) (Variables|Default|GetSpeedDecreaseMultiplyer)))
  (Variables|Default|SetIsAttacking true)
  (Variables|Default|SetCanAttack false)
  (Animation|PlayAnimMontage "/Game/BP/ABP/EnemyAttackMontage.EnemyAttackMontage" 1.0 "None"))

(fn WeaponHItStart
  (bind _weapon (Variables|Default|GetWeapon))
  (if (Utilities|IsValid _weapon)
    (Collision|SetCollisionEnabled (Variables|/Game/BP/Enemy/BP_EnemyWeapon.BP_EnemyWeapon_C|GetBox _weapon) "QueryOnly")))

(fn WeaponHitEnd
  (bind _weapon (Variables|Default|GetWeapon))
  (if (Utilities|IsValid _weapon)
    (Collision|SetCollisionEnabled (Variables|/Game/BP/Enemy/BP_EnemyWeapon.BP_EnemyWeapon_C|GetBox _weapon) "NoCollision")
    (Variables|/Game/BP/Enemy/BP_EnemyWeapon.BP_EnemyWeapon_C|SetIsPlayerHItted _weapon false)))

(fn AttackEndFunc
  (Variables|Default|SetIsAttacking false))

(fn SetAttackDelay
  (params (IsHit :type Boolean))
  (if IsHit
    (Variables|Default|SetAttackDelayTimer (Variables|Default|GetAttackSucessDelay))
    (else
      (Variables|Default|SetAttackDelayTimer (Variables|Default|GetAttackFailDelay)))))

(fn CheckinFront
  (params (Distance :type Float%20%28double-precision%29) (IsPlayerOnSight :type Boolean))
  (bind _returnvalue (Transformation|GetActorLocation))
  (bind _returnvalue_2 (Transformation|GetActorLocation))
  (bind _output_get (Variables|Default|SetCheckFrontTimer (+ (Utilities|Time|GetWorldDeltaSeconds) (Variables|Default|GetCheckFrontTimer))))
  (if (> _output_get 0.5)
    (Variables|Default|SetCheckFrontTimer 0.0)
    (if IsPlayerOnSight
      (bind (_outhit _returnvalue_3) (Collision|BoxTraceByChannel _returnvalue_2 (+ _returnvalue_2 (* (Math|Vector|Normalize (- (Transformation|GetActorLocation (Variables|Default|GetPlayer)) (Transformation|GetActorLocation))) Distance)) "32.000000,32.000000,32.000000" "0, 0, 0" "TraceTypeQuery1" true 0 "None"))
      (if _returnvalue_3
        (Utilities|Casting|CastToBP_SurvivorCharacter (.HitActor (Collision|BreakHitResult _outhit))
          (:then
            (Variables|Default|SetIsLookingPlayer true))
          (:CastFailed
            (Variables|Default|SetIsLookingPlayer false)
            (Variables|Default|SetIsPayerNear false)
            (if (< (Math|Vector|Distance(Vector) (.Location (Collision|BreakHitResult _outhit)) (Transformation|GetActorLocation)) (Variables|Default|GetReachBias))
              (bind _asbp_interactive (Utilities|Casting|CastToBP_Interactive (.HitActor (Collision|BreakHitResult _outhit)))
                (:then
                  (Transformation|SetActorRotation (Math|Rotator|MakeRotator 0.0 0.0 (.yaw (Math|Rotator|FindLookatRotation (Transformation|GetActorLocation) (Transformation|GetActorLocation _asbp_interactive)))))
                  (Variables|Default|SetPState "NewEnumerator5"))
                (:CastFailed
                  (Variables|Default|SetDestination "0, 0, 0")
                  (Variables|Default|SetPState "NewEnumerator0")))))))
      (else
        (bind (_outhit_2 _returnvalue_4) (Collision|BoxTraceByChannel _returnvalue (+ _returnvalue (* (Transformation|GetActorForwardVector) Distance)) "32.000000,32.000000,32.000000" "0, 0, 0" "TraceTypeQuery1" true 0 "None"))
        (if _returnvalue_4
          (if (< (Math|Vector|Distance(Vector) (.Location (Collision|BreakHitResult _outhit_2)) (Transformation|GetActorLocation)) (Variables|Default|GetReachBias))
            (bind _asbp_interactive_2 (Utilities|Casting|CastToBP_Interactive (.HitActor (Collision|BreakHitResult _outhit_2)))
              (:then
                (Transformation|SetActorRotation (Math|Rotator|MakeRotator 0.0 0.0 (.yaw (Math|Rotator|FindLookatRotation (Transformation|GetActorLocation) (Transformation|GetActorLocation _asbp_interactive_2)))))
                (Variables|Default|SetPState "NewEnumerator5"))
              (:CastFailed
                (Variables|Default|SetDestination "0, 0, 0")
                (Variables|Default|SetPState "NewEnumerator0")))))))))

(fn OnHitFlashLight
  (Variables|Default|SetPState "NewEnumerator4")
  (Variables|Default|SetIsStun true))

(fn KickHitBox
  (bind _returnvalue (Transformation|GetActorLocation))
  (bind (_outhits _returnvalue_2) (Class|KismetSystemLibrary|BoxTraceMulti _returnvalue (+ _returnvalue (* (Transformation|GetActorForwardVector) 1.5e+02)) "32.000000,64.000000,32.000000" "0, 0, 0" "TraceTypeQuery1" false 0 "ForDuration" true))
  (bind _array_element (Utilities|Array|ForEachLoopwithBreak _outhits)
    (:LoopBody
      (if _returnvalue_2
        (bind _asbp_interactive (Utilities|Casting|CastToBP_Interactive (.HitActor (Collision|BreakHitResult _array_element))))
        (Default|OnKillerInteract _asbp_interactive)))))

(fn KickEnd
  (Variables|Default|SetIsKicking false)
  (Variables|Default|SetPState "NewEnumerator0"))

(fn CheckPlayerDead
  (if (Variables|/Game/BP/Survivor/BP_SurvivorCharacter.BP_SurvivorCharacter_C|GetDead (Variables|Default|GetPlayer))
    (if (not (or (Utilities|Enum|Equal(Enum) (Variables|Default|GetPState) "NewEnumerator6") (Utilities|Enum|Equal(Enum) (Variables|Default|GetPState) "NewEnumerator7")))
      (Variables|Default|SetPState "NewEnumerator6"))))

(fn LiftingPlayer
  (Variables|Default|SetIsCarryPlayer true)
  (Transformation|AttachComponentToComponent (Variables|Default|GetPlayer) (Variables|Character|GetMesh) "PlayerSocket" "SnapToTarget" "SnapToTarget" "KeepWorld" true)
  ;[0.15 0.15 0.15 0.5] Temp
  (Collision|SetCollisionEnabled (Variables|/Script/Engine.Character|GetCapsuleComponent (Variables|Default|GetPlayer)) "NoCollision"))

(fn ResetBoolDatas
  (Utilities|FlowControl|Sequence
    (:then_0
      (Variables|Default|SetIsFindPlayer false)
      (Variables|Default|SetIsPayerNear false)
      (Variables|Default|SetIsLookingPlayer false))
    (:then_1
      (Variables|Default|SetCanAttack true)
      (Variables|Default|SetIsAttacking false)
      (Variables|Default|SetIsStun false))
    (:then_2
      (Variables|Default|SetIsKicking false)
      (Variables|Default|SetIsCarrying false)
      (Variables|Default|SetIsCarryPlayer false))))