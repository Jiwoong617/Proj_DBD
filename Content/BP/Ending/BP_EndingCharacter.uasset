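; BP_EndingCharacter is the actor for the game's ending, pairing the ending UI with automatic forward movement.
; On BeginPlay it creates WBP_EndingUI, adds it to the viewport, shows the mouse cursor and switches player 0 to UI-only input.
; Every Tick it offsets its location along its forward vector by Speed scaled by delta seconds, without sweeping for collision.
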(event EventBeginPlay
  (bind _returnvalue (Game|GetPlayerController 0))
  (bind _returnvalue_2 (UserInterface|CreateWidget "/Game/BP/Ending/WBP_EndingUI.WBP_EndingUI_C"))
  (bind _output_get (Variables|Default|SetEndUI _returnvalue_2))
  (UserInterface|Viewport|AddtoViewport _output_get 0)
  (Variables|/Script/Engine.PlayerController|SetbShowMouseCursor _returnvalue true)
  (Input|SetInputModeUIOnly _returnvalue 0 "DoNotLock" false))

(event Collision|EventActorBeginOverlap
  (params (OtherActor :type Actor%20Object%20Reference)))

(event EventTick
  (params (DeltaSeconds :type Float%20%28single-precision%29))
  (Transformation|SetActorLocation (+ (* DeltaSeconds (Variables|Default|GetSpeed) (Transformation|GetActorForwardVector)) (Transformation|GetActorLocation)) false false))

(fn ConstructionScript)