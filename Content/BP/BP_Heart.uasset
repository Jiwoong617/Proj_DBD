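; BP_Heart is a heart indicator actor that appears and beats according to its distance from the enemy.
; BeginPlay caches a BP_Enemy, and Tick hides the mesh whenever that enemy is beyond Distance.
; Within half that distance, Beating scales the mesh from OffsetScale to TargetScale using a hand-written elastic-out ease over elapsed time divided by Duration.
; The timer resets after one second, independent of Duration.
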(event EventBeginPlay
  (bind _returnvalue (Actor|GetActorOfClass "/Game/BP/Enemy/Trapper/BP_Enemy.BP_Enemy_C"))
  (Variables|Default|SetEnemy _returnvalue)
  (Variables|Default|Setc4 (/ (* (Math|Trig|GetPI) 2.0) 3.0)))

(event Collision|EventActorBeginOverlap
  (params (OtherActor :type Actor%20Object%20Reference)))

(event EventTick
  (params (DeltaSeconds :type Float%20%28single-precision%29))
  (bind _isnear (CallFunction|IsNear))
  (CallFunction|Beating _isnear))

(fn ConstructionScript)

(fn Beating
  (params (IsNear :type Boolean))
  (if (and IsNear (< (Math|Vector|Distance(Vector) (Transformation|GetActorLocation (Variables|Default|GetEnemy)) (Transformation|GetActorLocation)) (/ (Variables|Default|GetDistance) 2.0)))
    (bind _output_get (Variables|Default|SetElapsedTime (+ (Variables|Default|GetElapsedTime) (Utilities|Time|GetWorldDeltaSeconds))))
    (bind _value (CallFunction|ReturnElasticOutValue (/ _output_get (Variables|Default|GetDuration))))
    (Transformation|SetWorldScale3D (Variables|Default|GetStaticMesh) (Math|Vector|Lerp(Vector) (Variables|Default|GetOffsetScale) (Variables|Default|GetTargetScale) _value))
    (if (>= (Variables|Default|GetElapsedTime) 1.0)
      (Variables|Default|SetElapsedTime 0.0))))

(fn IsNear
  (bind _returnvalue (Transformation|GetActorLocation))
  (bind _enemy (Variables|Default|GetEnemy))
  (bind _distance (Variables|Default|GetDistance))
  (bind _returnvalue_2 (Transformation|GetActorLocation _enemy))
  (bind _returnvalue_3 (Math|Vector|Distance(Vector) _returnvalue_2 _returnvalue))
  (bind _returnvalue_4 (> _returnvalue_3 _distance))
  (Development|SetHiddeninGame (Variables|Default|GetStaticMesh) _returnvalue_4 false)
  (return (not _returnvalue_4)))

(fn ReturnElasticOutValue
  (params (ease :type Float%20%28double-precision%29))
  (if (or (== ease 1.0) (== ease 0.0))
    (return ease)
    (else
      (return (+ (* (Math|Float|Power 2.0 (* ease -1e+01)) (Math|Trig|Sin(Radians) (* (- (* ease 1e+01) 0.75) (Variables|Default|Getc4)))) 1.0)))))