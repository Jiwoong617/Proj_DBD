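; Repairable generator interactive for a survivor-versus-killer game, reporting completion to GM_MainGame to lower the generator count.
; Survivor overlap shows the repair widget and flags the character as repairing, while Tick accumulates progress during overlap.
; Killer interaction removes a tenth of progress, spawns an explosion and blocks repair until a delayed refresh.
; SetPlayerPos, uncalled here, snaps a target to one of three anchors, measuring two distances from world origin.
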(event OnComponentBeginOverlap(InterActRange)
  (params (OverlappedComponent :type Primitive%20Component%20Object%20Reference) (OtherActor :type Actor%20Object%20Reference) (OtherComp :type Primitive%20Component%20Object%20Reference) (OtherBodyIndex :type Integer) (bFromSweep :type Boolean) (SweepResult :type Hit%20Result%20Structure%20%28by%20ref%29))
  (bind _asbp_survivor_character (Utilities|Casting|CastToBP_SurvivorCharacter OtherActor))
  (Variables|/Game/BP/Survivor/BP_SurvivorCharacter.BP_SurvivorCharacter_C|Setbp_interactive _asbp_survivor_character self)
  (bind _output_get (Variables|Default|SetIsPlayerIn true))
  (if (and _output_get (Variables|Default|GetCanInteract))
    (Widget|SetVisibility (Variables|Default|GetGenUI) "Visible")
    (Variables|/Game/BP/Survivor/BP_SurvivorCharacter.BP_SurvivorCharacter_C|Setis%20Repairing _asbp_survivor_character true)))

(event OnComponentEndOverlap(InterActRange)
  (params (OverlappedComponent :type Primitive%20Component%20Object%20Reference) (OtherActor :type Actor%20Object%20Reference) (OtherComp :type Primitive%20Component%20Object%20Reference) (OtherBodyIndex :type Integer))
  (Utilities|Casting|CastToBP_SurvivorCharacter OtherActor)
  (Variables|Default|SetIsPlayerIn false)
  (Widget|SetVisibility (Variables|Default|GetGenUI) "Hidden")
  (Variables|/Game/BP/Survivor/BP_SurvivorCharacter.BP_SurvivorCharacter_C|Setis%20Repairing (stale OnComponentBeginOverlap(InterActRange) _asbp_survivor_character) false))

(event Custom|RefreshGenetator
  (Utilities|FlowControl|Delay (Variables|Default|GetGeneratorRefreshTime))
  (Variables|Default|SetCanInteract true))

(event EventBeginPlay
  (bind _returnvalue (UserInterface|CreateWidget "/Game/BP/MainUI/WBP_GeneratorUI.WBP_GeneratorUI_C"))
  (bind _output_get (Variables|Default|SetGenUI _returnvalue))
  (UserInterface|Viewport|AddtoViewport _output_get 0)
  (Widget|SetVisibility _output_get "Hidden"))

(event EventTick
  (params (DeltaSeconds :type Float%20%28single-precision%29))
  (bind _genui (Variables|Default|GetGenUI))
  (if (and (Variables|Default|GetIsPlayerIn) (Variables|Default|GetCanInteract))
    (bind _output_get (Variables|Default|SetTime (+ DeltaSeconds (Variables|Default|GetTime))))
    (if (> (/ _output_get (Variables|Default|GetRepairTime)) 1.0)
      (Widget|SetVisibility _genui "Hidden")
      (Variables|Default|SetCanInteract false)
      (bind _asgm_main_game (Utilities|Casting|CastToGM_MainGame (Game|GetGameMode)))
      (Default|DecreaseGeneratorCount _asgm_main_game)
      (else
        (Default|SetRepairValue _genui (/ _output_get (Variables|Default|GetRepairTime)))))))

(fn ConstructionScript
  (|CallParentFunction))

(fn OnKillerInteract
  (Variables|Default|SetCanInteract false)
  (bind _output_get (Variables|Default|SetTime (- (Variables|Default|GetTime) (* (Variables|Default|GetTime) 0.1))))
  (Default|SetRepairValue (Variables|Default|GetGenUI) (/ _output_get (Variables|Default|GetRepairTime)))
  (Niagara|SpawnSystematLocation "/Game/Effet/Generator_Boom.Generator_Boom" (Transformation|GetActorLocation))
  (CallFunction|RefreshGenetator))

(fn OnPlayerInteract
  (|CallParentFunction))

(fn SetPlayerPos
  (params (target :type BP%20Survivor%20Character%20Object%20Reference))
  (bind _actor_1 (Variables|Default|Getactor_1))
  (bind _actor_3 (Variables|Default|Getactor_3))
  (bind _actor_2 (Variables|Default|Getactor_2))
  (bind _capsulecomponent (Variables|/Script/Engine.Character|GetCapsuleComponent target))
  (bind _returnvalue (Transformation|GetWorldLocation _actor_2))
  (bind _returnvalue_2 (Transformation|GetWorldLocation _actor_3))
  (bind _returnvalue_3 (Transformation|GetWorldLocation _capsulecomponent))
  (bind _returnvalue_4 (Transformation|GetWorldLocation _actor_1))
  (bind _returnvalue_5 (Math|Vector|Distance(Vector) "0, 0, 0" _returnvalue_2))
  (bind _returnvalue_6 (Math|Vector|Distance(Vector) _returnvalue_3 _returnvalue_4))
  (bind _returnvalue_7 (Math|Vector|Distance(Vector) "0, 0, 0" _returnvalue))
  (bind _returnvalue_8 (Math|Float|Min(Float) _returnvalue_6 _returnvalue_7))
  (bind _returnvalue_9 (Math|Float|Min(Float) _returnvalue_8 _returnvalue_5))
  (LocalVariables|SetMindistance _returnvalue_9)
  (if (Math|Float|NearlyEqual(Float) _returnvalue_6 _returnvalue_8 0.01)
    (Transformation|SetActorLocation target (Transformation|GetWorldLocation (Variables|Default|Getactor_1)) false false)
    (bind _output_get (Variables|Default|SetUsed%20location "0, 0, 0"))
    (return _output_get)
    (elif (Math|Float|NearlyEqual(Float) _returnvalue_7 _returnvalue_8 0.01)
      (Transformation|SetActorLocation target (Transformation|GetWorldLocation (Variables|Default|Getactor_2)) false false)
      (bind _output_get_2 (Variables|Default|SetUsed%20location "0, 0, 0"))
      (return _output_get_2)
      (elif (Math|Float|NearlyEqual(Float) _returnvalue_5 _returnvalue_9 0.01)
        (Transformation|SetActorLocation target (Transformation|GetWorldLocation (Variables|Default|Getactor_3)) false false)
        (bind _output_get_3 (Variables|Default|SetUsed%20location "0, 0, 0"))
        (return _output_get_3)))))