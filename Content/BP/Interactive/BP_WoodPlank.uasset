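; BP_WoodPlank is an interactive plank that a survivor can topple and a killer can destroy.
; A trigger box flags overlap with BP_SurvivorCharacter and registers the plank as that character's interactive object.
; Survivor interaction runs the Spacebar event, which plays a timeline rolling the pivot and, after a short delay, enables plank collision, disabled at BeginPlay.
; Killer interaction simply destroys the actor.
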(event OnComponentBeginOverlap(TriggerBox)
  (params (OverlappedComponent :type Primitive%20Component%20Object%20Reference) (OtherActor :type Actor%20Object%20Reference) (OtherComp :type Primitive%20Component%20Object%20Reference) (OtherBodyIndex :type Integer) (bFromSweep :type Boolean) (SweepResult :type Hit%20Result%20Structure%20%28by%20ref%29))
  ;[0.15 0.15 0.15 0.5] Trigger box Interaction
  (bind _asbp_survivor_character (Utilities|Casting|CastToBP_SurvivorCharacter OtherActor))
  (Variables|Default|SetInteractive_WoodenPlanks true)
  (Variables|/Game/BP/Survivor/BP_SurvivorCharacter.BP_SurvivorCharacter_C|Setbp_interactive _asbp_survivor_character self))

(event OnComponentEndOverlap(TriggerBox)
  (params (OverlappedComponent :type Primitive%20Component%20Object%20Reference) (OtherActor :type Actor%20Object%20Reference) (OtherComp :type Primitive%20Component%20Object%20Reference) (OtherBodyIndex :type Integer))
  ;[0.15 0.15 0.15 0.5] Trigger box Interaction
  (Utilities|Casting|CastToBP_SurvivorCharacter OtherActor)
  (Variables|Default|SetInteractive_WoodenPlanks false))

(event Custom|Press"Spacebar"
  ;[0.15 0.15 0.15 0.5] Wooden_lnteractive
  (if (Variables|Default|GetInteractive_WoodenPlanks)
    (bind _woodenplanksani (Timeline|Timeline Play)
      (:Update
        (Transformation|SetRelativeRotation (Variables|Default|Getpivot) (Math|Rotator|MakeRotator _woodenplanksani 0.0 0.0) false false)
        (Utilities|FlowControl|Delay 0.5)
        (Collision|SetCollisionEnabled (Variables|Default|GetWoodenPlanks) "QueryAndPhysics")))))

(event EventBeginPlay
  (Collision|SetCollisionEnabled (Variables|Default|GetWoodenPlanks) "NoCollision"))

(event Collision|EventActorBeginOverlap
  (params (OtherActor :type Actor%20Object%20Reference)))

(event EventTick
  (params (DeltaSeconds :type Float%20%28single-precision%29))
  (|CallParentFunction DeltaSeconds) ; This node is disabled and will not be called.\nDrag off pins to build functionality.
)

(fn ConstructionScript
  (|CallParentFunction))

(fn OnKillerInteract
  (Actor|DestroyActor))

(fn OnPlayerInteract
  (CallFunction|Press"Spacebar"))