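; BP_VaultTrigger is a trigger actor that moves a survivor across a vault spot by teleporting it.
; Space Bar press and release events on the trigger set and clear a PressVault flag, which is checked only when something begins overlapping the Box.
; If the flag is set, a BP_SurvivorCharacter snaps without sweep to whichever is nearer, SetVaultPos or SetInvertVaultPos, with no animation.
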(event OnComponentBeginOverlap(Box)
  (params (OverlappedComponent :type Primitive%20Component%20Object%20Reference) (OtherActor :type Actor%20Object%20Reference) (OtherComp :type Primitive%20Component%20Object%20Reference) (OtherBodyIndex :type Integer) (bFromSweep :type Boolean) (SweepResult :type Hit%20Result%20Structure%20%28by%20ref%29))
  ;[0.15 0.15 0.15 0.5] 위치 변환_trigger 와 캐릭터의 거리
  (if (stale Input|KeyboardEvents|SpaceBar _output_get)
    (bind _asbp_survivor_character (Utilities|Casting|CastToBP_SurvivorCharacter OtherActor))
    (if (< (Math|Vector|Distance(Vector) (Transformation|GetActorLocation _asbp_survivor_character) (Transformation|GetWorldLocation (Variables|Default|GetSetVaultPos))) (Math|Vector|Distance(Vector) (Transformation|GetActorLocation _asbp_survivor_character) (Transformation|GetWorldLocation (Variables|Default|GetSetInvertVaultPos))))
      (Transformation|SetActorLocation _asbp_survivor_character (Transformation|GetWorldLocation (Variables|Default|GetSetVaultPos)) false false)
      (else
        (Transformation|SetActorLocation _asbp_survivor_character (Transformation|GetWorldLocation (Variables|Default|GetSetInvertVaultPos)) false false)))))

(event EventBeginPlay)

(event Collision|EventActorBeginOverlap
  (params (OtherActor :type Actor%20Object%20Reference)))

(event EventTick
  (params (DeltaSeconds :type Float%20%28single-precision%29)))

(event Input|KeyboardEvents|SpaceBar
  (params (Key :type Key%20Structure :default "None"))
  (:Pressed
    (bind _output_get (Variables|Default|SetPress_Vault true)))
  (:Released
    (Variables|Default|SetPress_Vault false)))

(fn ConstructionScript)