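; Main game mode that drives the match through start, gaming and end states via SwtichGameState.
; Start creates the WBP_Main HUD and fades the camera in, then switches to gaming after a delay; that state runs no logic here.
; End fades the camera out and opens the end level.
; SetPlayerCondition and DecreaseGeneratorCount simply forward player state and generator updates to the HUD.
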(event Custom|OnGameEndEvent
  (CameraFades|StartCameraFade :self (Game|GetPlayerCameraManager 0) :ToAlpha 1.0 :Duration 2.0 :bHoldWhenFinished true)
  (Utilities|FlowControl|Delay 2.0)
  (Game|OpenLevel(byName) (Variables|Default|GetEndLevelName)))

(event Custom|OnGameStart
  (bind _returnvalue (UserInterface|CreateWidget "/Game/BP/MainUI/WBP_Main.WBP_Main_C"))
  (bind _output_get (Variables|Default|SetMainUI _returnvalue))
  (UserInterface|Viewport|AddtoViewport _output_get 0)
  (CameraFades|StartCameraFade :self (Game|GetPlayerCameraManager 0) :FromAlpha 1.0 :Duration 1.0 :bHoldWhenFinished true)
  (Utilities|FlowControl|Delay 1.0)
  (Utilities|FlowControl|Delay 5.0)
  (CallFunction|SwtichGameState "NewEnumerator1"))

(event EventBeginPlay
  (CallFunction|SwtichGameState "NewEnumerator0"))

(event EventTick
  (params (DeltaSeconds :type Float%20%28single-precision%29)))

(fn ConstructionScript)

(fn SwtichGameState
  (params (GameState :type EGameMode%20Enum :default "NewEnumerator0"))
  (bind _output_get (Variables|Default|SetState GameState))
  (switch Utilities|FlowControl|Switch|SwitchonEGameMode _output_get
    (:NewEnumerator0
      (CallFunction|OnGameStart))
    (:NewEnumerator2
      (CallFunction|OnGameEndEvent))))

(fn SetPlayerCondition
  (params (state :type EPlayerState%20Enum :default "NewEnumerator0"))
  (Default|SetPlayerCondition (Variables|Default|GetMainUI) state))

(fn DecreaseGeneratorCount
  (Default|DecreaseGeneratorCount (Variables|Default|GetMainUI)))